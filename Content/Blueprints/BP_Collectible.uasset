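; BP_Collectible is a pickup actor that spins and shakes in place until the player touches it.
; Tick adds a small local rotation and plays the Shake timeline, whose track feeds a local position offset on each update.
; Overlap by player pawn 0 plays a 2D sound, spawns a particle emitter at the Sphere's location and destroys the actor.
; The pickup itself awards no score or item.
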(event `self.ReceiveActorBeginOverlap`
  (params (OtherActor :type "Actor Object Reference"))
  (if (== OtherActor (`GameplayStatics.GetPlayerPawn` 0))
    (`GameplayStatics.PlaySound2D` "/Game/Audio/Randomize13.Randomize13" 1.0 1.0 0.0 null null)
    (`GameplayStatics.SpawnEmitterAtLocation` (`self.Emitter`) (`SceneComponent.K2_GetComponentLocation` (`self.Sphere`)))
    (`self.K2_DestroyActor`)))

(event `self.ReceiveTick`
  (params (DeltaSeconds :type "Float (single-precision)"))
  (`self.K2_AddActorLocalRotation` (struct :`Yaw` 0.5))
  (bind (_direction _newtrack_0) (`Timeline|Shake`)
    (:`Update`
      (`self.K2_AddActorLocalOffset` _newtrack_0))))

(fn `UserConstructionScript`)