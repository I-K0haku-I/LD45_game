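; BP_DoorKey is a pickup key that grants door access to the player.
; When an FPS_Controller overlaps it, it adds its Key entries to that controller, notifies each registered owner door via KeyTaken, then destroys itself.
; Doors register through AddOwner, and the construction script tints the key sphere with a dynamic material using the Color variable.
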(event `self.ReceiveActorBeginOverlap`
  (params (OtherActor :type "Actor Object Reference"))
  (bind _asfps_controller (cast `/Game/Blueprints/FPS_Controller` OtherActor))
  (for _array_element (`self.Key`)
    (`/Game/Blueprints/FPS_Controller.AddKey` _asfps_controller _array_element))
  (for _array_element_2 (`self.OwnerDoor`)
    (`/Game/Blueprints/BPI_Door.KeyTaken` _array_element_2 self))
  (`self.K2_DestroyActor`))

(fn `AddOwner`
  (params (`The Owner` :type "/Game/Blueprints/BPI_Door Interface"))
  (`KismetArrayLibrary.Array_Add` (`self.OwnerDoor`) `The Owner`))

(fn `UserConstructionScript`
  (bind _returnvalue (`PrimitiveComponent.CreateDynamicMaterialInstance` (`self.Key Sphere`) 0 "/Game/Materials/M_DoorClay1.M_DoorClay1" "None"))
  (`MaterialInstanceDynamic.SetVectorParameterValue` _returnvalue "Color" (`self.Color`)))