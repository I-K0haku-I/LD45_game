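; BP_MechanicCheck is a one-shot trigger that reveals an obstacle and shows an instruction when the player reaches it.
; On BeginPlay it hides the referenced Obstacle and disables its collision.
; The first overlap by the player pawn clears IsReady, restores the obstacle's visibility and collision, and writes Instruction into the WBP_WorldText of its Widget component.
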(event `self.ReceiveBeginPlay`
  (bind _obstacle (`self.Obstacle`))
  ;[1 1 1] disable obstacle
  (`self.SetActorHiddenInGame` _obstacle true)
  (`self.SetActorEnableCollision` _obstacle false))

(event `self.ReceiveActorBeginOverlap`
  (params (OtherActor :type "Actor Object Reference"))
  (bind _obstacle (`self.Obstacle`))
  ;[1 1 1] Trigger only once
  (if (and (== OtherActor (`GameplayStatics.GetPlayerPawn` 0)) (`self.IsReady`))
    (set `self.IsReady` false)
    ;[1 1 1] enable obstacle
    (`self.SetActorHiddenInGame` _obstacle false)
    (`self.SetActorEnableCollision` _obstacle true)
    (bind _aswbp_world_text (cast `/Game/Blueprints/WBP_WorldText` (`WidgetComponent.GetUserWidgetObject` (`self.Widget`))))
    (set `/Game/Blueprints/WBP_WorldText.Text` (`self.Instruction`) _aswbp_world_text)))

(fn `Test`)

(fn `UserConstructionScript`)