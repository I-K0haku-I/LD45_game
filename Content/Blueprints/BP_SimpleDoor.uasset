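; BP_SimpleDoor is a door that snaps between opened and closed marker transforms and attempts to auto-close after a delay.
; ToggleDoor checks CanOpenByController, which just returns the CanOpen flag, then moves DoorMesh with sweep.
; It sets IsCurrentlyOpen from mesh visibility rather than the requested state.
; Tick counts CloseUntil down while that flag is true, calling close below zero, and otherwise resets it to CloseTime.
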(event `self.ReceiveTick`
  (params (DeltaSeconds :type "Float (single-precision)"))
  (if (`self.isCurrentlyOpen`)
    (bind _output_get (set `self.CloseUntil` (- (`self.CloseUntil`) DeltaSeconds)))
    (if (< _output_get 0.0)
      (`self.ToggleDoor` null false))
    (else
      (set `self.CloseUntil` (`self.CloseTime`)))))

(fn `CanOpenByController`
  (params (Controller :type "/Game/Blueprints/FPS_Controller Object Reference"))
  (returns (CanOpen :type Boolean))
  (return (`self.CanOpen`)))

(fn `IsOpen`
  (returns (isOpen :type Boolean))
  (return (`self.isCurrentlyOpen`)))

(fn `ToggleDoor`
  (params (Controller :type "/Game/Blueprints/FPS_Controller Object Reference") (Open :type Boolean))
  (returns (HasOpened :type Boolean))
  (bind _doormesh (`self.DoorMesh`))
  (bind _canopen (`self.CanOpenByController` Controller))
  (if _canopen
    (`SceneComponent.K2_SetRelativeTransform` _doormesh (select `bool` Open :`false` (`SceneComponent.GetRelativeTransform` (`self.ClosedPosition`)) :`true` (`SceneComponent.GetRelativeTransform` (`self.OpenedPosition`))) true false)
    (bind _output_get (set `self.isCurrentlyOpen` (`SceneComponent.bVisible` _doormesh)))
    (return _output_get)))

(fn `UserConstructionScript`)