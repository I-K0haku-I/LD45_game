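; BP_UnlockCollectible is a child collectible that unlocks an ability on the player character when overlapped.
; On overlap it runs the parent logic, then enables the ability given by its Type variable on player pawn 0, cast to FPS_Controller, without checking the overlapping actor itself.
; Its construction script extends the parent's by setting an unlock-specific sphere material and particle emitter.
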(event `self.ReceiveActorBeginOverlap`
  (params (OtherActor :type "Actor Object Reference"))
  (`parent.ReceiveActorBeginOverlap` OtherActor)
  ;[1 1 1] Added unlocking of abilities on character - DerpyNewbie
  (bind _asfps_controller (cast `/Game/Blueprints/FPS_Controller` (`GameplayStatics.GetPlayerPawn` 0)))
  (`/Game/Blueprints/FPS_Controller.ToggleAbility` _asfps_controller (`self.Type`) true))

(event `self.ReceiveTick`
  (params (DeltaSeconds :type "Float (single-precision)"))
  (`parent.ReceiveTick` DeltaSeconds))

(fn `UserConstructionScript`
  (`parent.UserConstructionScript`)
  (`PrimitiveComponent.SetMaterial` (`self.Sphere`) 1 "/Game/Materials/M_UnlockCollectible_inst.M_UnlockCollectible_inst")
  (set `self.Emitter` "/Game/Particles/PS_UnlockCollectible.PS_UnlockCollectible"))